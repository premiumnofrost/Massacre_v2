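; Base character Blueprint for the MACS GAS combat system, shared by players and AI.
; It starts common weapon and effect-loop abilities on possession, then adds a nameplate, HUD attribute binding and trace component at BeginPlay.
; Server events set replicated state; OnReps apply collision, speed, physics, team tint, hit reactions and scoring.
; It also handles hit FX, respawn via GameMode or AI spawn, and demo trigger-box team assignment.
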(event EventPossessed
  (params (NewController :type Controller%20Object%20Reference))
  (bind _returnvalue (Class|MACSCharacter|GetAbilitySystemComponent))
  ;[1 1 1] Setup Character when Possessed on server and at BeginPlay
  (Utilities|FlowControl|DoOnce false
    (:Completed
      ;;[1 1 1] Set the WeaponClass as Commun
      (GameplayEffects|ApplyGameplayEffectToSelf :self _returnvalue :GameplayEffectClass "/Game/MACS/GAS/Effects/States/WeaponClass/GE_MACS_WeaponClass_Commun.GE_MACS_WeaponClass_Commun_C")
      ;;[1 1 1] Handle Passives regens/degens and Crawling/Death State
      (Abilities|TryActivateAbilitybyClass _returnvalue "/Game/MACS/GAS/Abilities/Commun/GA_MACS_Commun_GameplayEffectsLoop.GA_MACS_Commun_GameplayEffectsLoop_C" true))))

(event EventBeginPlay
  ;[1 1 1] Setup Character when Possessed on server and at BeginPlay
  (Utilities|FlowControl|Sequence
    (:then_0
      ;;[1 1 1] Only players can creates HUD
      (Utilities|FlowControl|Delay 0.3)
      (bind _result (MACS|CreateNameplateWidget))
      (if _result
        ;;[1 1 1] Setup Name and AttributeSet on UI on players
        (if (Pawn|IsPlayerControlled)
          (MACS|SetupAttributeSet)
          (MACS|SetupName))))
    (:then_1
      (MACS|StoreDefaultMattoResetTeamID))
    (:then_2
      (Game|AddComponentbyClass "/Game/MACS/Classes/Components/BP_MACS_TraceComp.BP_MACS_TraceComp_C"))))

(event EventDestroyed
  ;[1 1 1] TryToDropAllItems when destroyed
  (Ability|SendGameplayEventtoActor self "(TagName=\"MACS_GAS.Abilities.Events.SetWeaponClass.TryToDropAll\")"))

(fn ConstructionScript)

(fn SetPawnCollisionResponse
  ;[1 1 1] Set pawn collision response by the server
  (Collision|SetCollisionResponsetoChannel (Variables|Default|GetCapsuleComponent) "ECC_Pawn" (Variables|MACS|Demo|GetPawnResponse)))

(fn OnRepPawnResponse
  (MACS|SetPawnCollisionResponse))

(fn SetupAttributeSet
  ;[1 1 1] Try to Setup AttributeSet on Hud
  (bind _asplayer_controller (Utilities|Casting|CastToPlayerController (Pawn|GetController)))
  (bind _asbp_macs_hud (Utilities|Casting|CastToBP_MACS_HUD (HUD|GetHUD _asplayer_controller)))
  (Variables|/Game/MACS/UI/WB_MACS_CharData.WB_MACS_CharData_C|SetAttributeSetRef (Variables|/Game/MACS/UI/WB_MACS_UI.WB_MACS_UI_C|GetBP_MACS_GAS_CharData (Variables|/Game/MACS/UI/BP_MACS_HUD.BP_MACS_HUD_C|GetUI _asbp_macs_hud)) (Variables|Default|GetMACS_AttributeSet))
  (Variables|/Game/MACS/UI/WB_MACS_CharData.WB_MACS_CharData_C|SetPawnRef (Variables|/Game/MACS/UI/WB_MACS_UI.WB_MACS_UI_C|GetBP_MACS_GAS_CharData (Variables|/Game/MACS/UI/BP_MACS_HUD.BP_MACS_HUD_C|GetUI _asbp_macs_hud)) self)
  (return))

(fn Respawn
  ;[1 1 1] Only Authority
  (Networking|SwitchHasAuthority
    (:Authority
      ;[1 1 1] Is a player controlled or AI controlled?
      (if (Pawn|IsPlayerControlled)
        (MACS|RestartPlayer)
        (else
          ;[1 1 1] Spawn new AI with the same TeamID
          (bind _outactors (Actor|GetAllActorsOfClass "/Game/MACS/Classes/BP_MACS_SpawnRef.BP_MACS_SpawnRef_C"))
          (for _array_element _outactors
            (if (== (Variables|/Game/MACS/Classes/BP_MACS_SpawnRef.BP_MACS_SpawnRef_C|GetTeamIdRef _array_element) (Variables|MACS|GetTeamID))
              (bind _returnvalue (AI|SpawnAIFromClass (Utilities|GetClass self) "/Game/MACS/AI/BT_MACS_Demo.BT_MACS_Demo" (.location (Transformation|GetActorTransform _array_element)) (.rotation (Transformation|GetActorTransform _array_element)) true 0))
              (Class|BPIMACSCharacter|SetTeamID(Message) _returnvalue (Variables|MACS|GetTeamID)))))))))

(fn OnRepSimulatePhysics
  (Physics|SetSimulatePhysics (Variables|Character|GetMesh) (Variables|MACS|GetSimulatePhysics)))

(fn OnRepMaxWalkSpeed
  (Variables|/Script/Engine.CharacterMovementComponent|SetMaxWalkSpeed (Variables|Character|GetCharacterMovement) (Variables|MACS|GetMaxWalkSpeed)))

(fn OnRepPlayerResponsetoInvWall
  (if (Variables|MACS|Demo|GetPlayerResponseToInvWall)
    (Collision|SetCollisionResponsetoChannel (Variables|Default|GetCapsuleComponent) "ECC_Destructible" "ECR_Ignore")))

(fn CreateNameplateWidget
  ;[1 1 1] Create Widget Nameplate
  (bind _returnvalue (AddComponent|AddWidgetComponent false (Math|Transform|MakeTransform "0, 0,100.000000" "0, 0, 0" "1.000000,1.000000,1.000000")))
  (Utilities|IsValid _returnvalue
    (:Is%20Valid
      (Class|WidgetComponent|SetWidgetSpace _returnvalue "Screen")
      (bind _returnvalue_2 (UserInterface|CreateWidget "/Game/MACS/UI/WB_MACS_Nameplate.WB_MACS_Nameplate_C" 0 self))
      (Utilities|IsValid _returnvalue_2
        (:Is%20Valid
          (UserInterface|SetWidget _returnvalue _returnvalue_2)
          (return true))
        (:Is%20Not%20Valid
          _)))
    (:Is%20Not%20Valid
      _))
  (return false))

(fn SetupName
  (if (Pawn|IsPlayerControlled)
    (bind _asbp_mads_world_character (Utilities|Casting|CastToBP_MADS_WorldCharacter (Pawn|GetControlledPawn (Game|GetPlayerController 0))))
    (Variables|MACS|SetPlayerName (.name (Variables|/Game/MADS/Base/BP_MADS_WorldCharacter.BP_MADS_WorldCharacter_C|GetCharData _asbp_mads_world_character)))
    (else
      (Variables|MACS|SetPlayerName "AI"))))

(fn OnRepTeamID
  (bind _mesh (Variables|Character|GetMesh))
  ;[1 1 1] DEMO: Set Char Color by the TeamID if != -1
  (if (== (Variables|MACS|GetTeamID) -1)
    (for (_array_element _array_index) (Variables|MACS|Demo|GetDefaultMaterials)
      (Rendering|Material|SetMaterial (Variables|Character|GetMesh) _array_index (.materialinterface _array_element)))
    (else
      (for (_array_element_2 _array_index_2) (Variables|/Script/Engine.SkeletalMesh|GetMaterials (Variables|/Script/Engine.SkeletalMeshComponent|GetSkeletalMeshAsset _mesh))
        (bind _returnvalue (Rendering|Material|CreateDynamicMaterialInstance (.materialinterface _array_element_2) "None" "None" :!class /Script/Engine.KismetMaterialLibrary))
        (Rendering|Material|SetVectorParameterValue _returnvalue "Tint" (Utilities|Select :Index (Variables|MACS|GetTeamID) :Option%200 "" :Option%201 "(R=1.000000,G=0.000000,B=0.000000,A=1.000000)" :Option%202 "(R=0.000000,G=2.000000,B=0.000000,A=1.000000)" :Option%203 "(R=0.000000,G=0.000000,B=3.000000,A=1.000000)" :Option%204 "(R=1.000000,G=1.000000,B=0.000000,A=1.000000)" :Option%205 "(R=1.000000,G=0.000000,B=1.000000,A=1.000000)" :Option%206 "(R=0.000000,G=1.000000,B=1.000000,A=1.000000)") :!class /Script/Engine.MaterialInstanceDynamic)
        (Rendering|Material|SetMaterial _mesh _array_index_2 _returnvalue)))))

(fn DemoSetTeamIdwhenBeginOverlap
  (params (ActorRef :type Actor%20Object%20Reference))
  (bind _returnvalue (Utilities|GetDisplayName ActorRef))
  (if (Utilities|String|Contains _returnvalue "TriggerBox_Blue")
    (if (== (Variables|MACS|GetTeamID) -1)
      (Variables|MACS|SetTeamID 3)
      (return))
    (elif (Utilities|String|Contains _returnvalue "TriggerBox_Red")
      (if (== (Variables|MACS|GetTeamID) -1)
        (Variables|MACS|SetTeamID 1)))))

(fn DemoBeginOverlapDojo
  (params (ActorRef :type Actor%20Object%20Reference))
  (if (and (Pawn|IsPlayerControlled) (Ability|HasAuthority))
    (bind _astrigger_box (Utilities|Casting|CastToTriggerBox ActorRef))
    (Utilities|FlowControl|Sequence
      (:then_0
        (MACS|Demo|DemoSetTeamIdwhenBeginOverlap _astrigger_box))
      (:then_1
        (if (Utilities|String|Contains (Utilities|GetDisplayName _astrigger_box) "TriggerBox_Dojo")
          (Variables|MACS|Demo|SetInDojo true))))))

(fn DemoEndOverlapDojo
  (params (ActorRef :type Actor%20Object%20Reference))
  (if (and (Pawn|IsPlayerControlled) (Ability|HasAuthority))
    (bind _astrigger_box (Utilities|Casting|CastToTriggerBox ActorRef))
    (Utilities|FlowControl|Sequence
      (:then_0
        (MACS|Demo|DemoResetTeamIdwhenEndOverlap _astrigger_box))
      (:then_1
        (MACS|Demo|DemoResetDojoState _astrigger_box)))))

(fn DemoResetTeamIdwhenEndOverlap
  (params (ActorRef :type Actor%20Object%20Reference))
  (bind _returnvalue (Utilities|GetDisplayName ActorRef))
  (if (and (or (Utilities|String|Contains _returnvalue "TriggerBox_Blue") (Utilities|String|Contains _returnvalue "TriggerBox_Red")) (not (Variables|MACS|Demo|GetInDojo)))
    (Variables|MACS|SetTeamID -1)))

(fn DemoResetDojoState
  (params (ActorRef :type Actor%20Object%20Reference))
  (if (Utilities|String|Contains (Utilities|GetDisplayName ActorRef) "TriggerBox_Dojo")
    (Variables|MACS|Demo|SetInDojo false)))

(fn StoreDefaultMattoResetTeamID
  ;[1 1 1] Store the default materials to when reset TeamID
  (Variables|MACS|Demo|SetDefaultMaterials (Variables|/Script/Engine.SkeletalMesh|GetMaterials (Variables|/Script/Engine.SkeletalMeshComponent|GetSkeletalMeshAsset (Variables|Character|GetMesh)))))

(fn RestartPlayer
  ;[1 1 1] Respawn restarting on GM
  (bind _output_get (LocalVariables|SetControllerRef (Pawn|GetController)))
  (Actor|DestroyActor)
  (Class|GameModeBase|RestartPlayer (Game|GetGameMode) _output_get)
  (Default|SelectNewCharacteronServer (Variables|/Game/MACS/Classes/BP_MACS_PC.BP_MACS_PC_C|GetBP_MADS_Comp (.AsBP%20MACS%20PC (Utilities|Casting|CastToBP_MACS_PC _output_get)))))

(fn OnRepHitReaction
  (Utilities|FlowControl|Sequence
    (:then_0
      (if (Pawn|IsLocallyControlled)
        (Abilities|TryActivateAbilitybyClass (Variables|Default|GetMACS_AbilitySystemComponent) "/Game/MACS/GAS/Abilities/Commun/GA_MACS_Commun_HitReactions.GA_MACS_Commun_HitReactions_C" true)))
    (:then_1
      (Utilities|IsValid (.instigator (Variables|MACS|Runtime|GetHitReaction))
        (:Is%20Valid
          ;[1 1 1] Send Score to player and investigator
          (if (Math|Boolean|ANDBoolean (not (CallFunction|GameplayTagCheck self "(TagName=\"MACS_GAS.Abilities.States.Crawling\")")) (<= (.ReturnValue (Class|AbilitySystemComponent|GetGameplayAttributeValue (Variables|Default|GetMACS_AbilitySystemComponent) "(AttributeName=\"Health\",Attribute=/Script/MACS.MACS_AttributeSet:Health,AttributeOwner=\"/Script/CoreUObject.Class'/Script/MACS.MACS_AttributeSet'\")")) 0.0) (!= (.instigator (Variables|MACS|Runtime|GetHitReaction)) self))
            (Default|ScoreAddDeath self)
            (bind _asbp_mads_world_character (Utilities|Casting|CastToBP_MADS_WorldCharacter (.instigator (Variables|MACS|Runtime|GetHitReaction))))
            (Default|ScoreAddKill _asbp_mads_world_character)))))))

(fn MCPlayFx
  (params (Hit :type Hit%20Result%20Structure) (Actor :type Actor%20Object%20Reference))
  (bind (_bblockinghit _binitialoverlap _time _distance _location _impactpoint _normal _impactnormal _physmat _hitactor _hitcomponent) (Collision|BreakHitResult Hit))
  (bind (_bblockinghit_2 _binitialoverlap_2 _time_2 _distance_2 _location_2 _impactpoint_2 _normal_2 _impactnormal_2 _physmat_2 _hitactor_2) (Collision|BreakHitResult Hit))
  (if (and (== (Utilities|GetClass _hitcomponent) "/Script/Engine.SkeletalMeshComponent") (not (CallFunction|GameplayTagCheck _hitactor "(TagName=\"MACS_GAS.Abilities.States.Dead\")")))
    ;[1 1 1] If target are in the valid defense mode, make fx like eviroment
    (if (not (CallFunction|IsValidDefenseMode _hitactor_2 Actor))
      (Utilities|FlowControl|Sequence
        (:then_0
          (Niagara|SpawnSystematLocation (.OutItem (Utilities|Array|Random (LocalVariables|GetParticleWhenPawnHitted))) _location_2))
        (:then_1
          (bind _soundwhenpawnhitted (LocalVariables|GetSoundWhenPawnHitted)
            (:then
              (Audio|SpawnSoundatLocation _soundwhenpawnhitted _location_2 "0, 0, 0" 1.0 1.0 0.0 0 0)
              (return true))
            (:else))))
      (else
        (Utilities|FlowControl|Sequence :!label _label
          (:then_0
            (bind _particlewhenenvironmenthitted (LocalVariables|GetParticleWhenEnvironmentHitted)
              (:then
                (Effects|SpawnEmitteratLocation _particlewhenenvironmenthitted _location_2 "0, 0, 0" "2.000000,2.000000,2.000000" true "AutoRelease"))
              (:else)))
          (:then_1
            (bind _soundwhenenvironmenthitted (LocalVariables|GetSoundWhenEnvironmentHitted)
              (:then
                (Audio|SpawnSoundatLocation _soundwhenenvironmenthitted _location_2 "0, 0, 0" 0.25 1.0 0.0 0 0)
                (return true))
              (:else))))))
    (else
      (goto _label))))

(event Custom|SetInDojoOnServer
  (params (InDojo :type Boolean))
  ;[1 1 1] MACS Demo/Features
  (Variables|MACS|Demo|SetInDojo InDojo))

(event Custom|RespawnOnServer
  ;[1 1 1] MACS Demo/Features
  (MACS|Demo|Respawn))

(event Custom|SetMaxWalkSpeedOnServer
  (params (MaxWalkSpeed :type Float%20%28double-precision%29))
  ;[1 1 1] MACS Demo/Features
  (Variables|MACS|SetMaxWalkSpeed MaxWalkSpeed))

(event Custom|SetOrientToMovementServer
  (params (Orient%20Rotation%20to%20Movement :type Boolean))
  ;[1 1 1] MACS Demo/Features
  (Variables|/Script/Engine.CharacterMovementComponent|SetbOrientRotationToMovement (Variables|Character|GetCharacterMovement) Orient%20Rotation%20to%20Movement))

(event Custom|SetCapsuleCollisionOnAll
  (params (Channel :type ECollisionChannel%20Enum :default "ECC_Pawn") (NewResponse :type ECollisionResponse%20Enum :default "ECR_Overlap"))
  ;[1 1 1] MACS Demo/Features
  (Collision|SetCollisionResponsetoChannel (Variables|Default|GetCapsuleComponent) Channel NewResponse))

(event Custom|SetTeamIdOnServer
  (params (TeamID :type Integer))
  ;[1 1 1] MACS Demo/Features
  (Variables|MACS|SetTeamID TeamID))

(event Custom|SetShowDebugTrace
  (params (ShowDebugTrace :type Boolean))
  ;[1 1 1] MACS Demo/Features
  (Variables|MACS|Demo|SetShowDebugTrace ShowDebugTrace))

(event Custom|SetPawnCollisionResponseOnServer
  (params (PawnResponse :type ECollisionResponse%20Enum :default "ECR_Ignore"))
  ;[1 1 1] MACS Demo/Features
  (Variables|MACS|Demo|SetPawnResponse PawnResponse))

(event Custom|SetSimulatePhysicsOnServer
  (params (SimulatePhysics :type Boolean))
  ;[1 1 1] MACS Demo/Features
  (Variables|MACS|SetSimulatePhysics SimulatePhysics))

(event Custom|SetDirectionToDashOrEscapeOnServer
  (params (DirectionToDashOrEscape :type E_MACS_Direction%20Enum :default "NewEnumerator0"))
  ;[1 1 1] MACS Demo/Features
  (Variables|MACS|SetDirectionToDashOrEscape DirectionToDashOrEscape))

(event Custom|SpawnEmmiterOnClient
  (params (Hit :type Hit%20Result%20Structure) (Actor :type Actor%20Object%20Reference))
  (CallFunction|MCPlayFx Hit Actor))

(event Custom|SetHitReactionOnServer
  (params (S_MACS_HitReaction :type S%20MACS%20Hit%20Reaction%20Structure))
  ;[1 1 1] MACS Demo/Features
  (Variables|MACS|Runtime|SetHitReaction S_MACS_HitReaction))

(event Custom|SendGameplayEventToOwnerOnServer
  (params (EventTag :type Gameplay%20Tag%20Structure) (Payload :type Gameplay%20Event%20Data%20Structure))
  ;[1 1 1] MACS Demo/Features
  (Ability|SendGameplayEventtoActor self EventTag Payload))

(event EventSendGameplayEvent
  (params (GameplayTag :type Gameplay%20Tag%20Structure) (Payload :type Gameplay%20Event%20Data%20Structure))
  (CallFunction|SendGameplayEventtoOwneronServer GameplayTag Payload))

(event EventSetTeamID
  (params (TeamID :type Integer))
  (CallFunction|SetTeamIdonServer TeamID))

(event EventSetCapsuleCollision
  (params (Channel :type ECollisionChannel%20Enum :default "ECC_WorldStatic") (NewResponse :type ECollisionResponse%20Enum :default "ECR_Ignore"))
  (CallFunction|SetCapsuleCollisiononAll Channel NewResponse))

(event EventSetMAxWalkSpeed
  (params (NewMaxWalkSpeed :type Float%20%28double-precision%29))
  (CallFunction|SetMaxWalkSpeedonServer NewMaxWalkSpeed))

(event EventSetHitReaction
  (params (MACS_HitReaction :type S%20MACS%20Hit%20Reaction%20Structure))
  (CallFunction|SetHitReactiononServer MACS_HitReaction))

(event EventSetDirectiontoDashorEscape
  (params (DirectionToDashOrEscape :type E_MACS_Direction%20Enum :default "NewEnumerator0"))
  (CallFunction|SetDirectiontoDashorEscapeonServer DirectionToDashOrEscape))

(event EventISetPawnCollisionResponse
  (params (PawnCollisionResponse :type ECollisionResponse%20Enum :default "ECR_Ignore"))
  (CallFunction|SetPawnCollisionResponseonServer PawnCollisionResponse))

(event EventSetSimulatePhysics
  (params (SimulatePhysics :type Boolean))
  (CallFunction|SetSimulatePhysicsonServer SimulatePhysics))

(event EventSetRotationOrienttoMovement
  (params (Orient :type Boolean))
  (CallFunction|SetOrienttoMovementServer Orient))

(event EventIRespawn
  (CallFunction|RespawnonServer))

(fn GetDebugTrace
  (return (Variables|MACS|Demo|GetShowDebugTrace)))

(fn GetDirectiontoDashorEscape
  (return (Variables|MACS|GetDirectionToDashOrEscape)))

(fn GetHitReaction
  (return (Variables|MACS|Runtime|GetHitReaction)))

(fn GetTeamID
  (return (Variables|MACS|GetTeamID)))