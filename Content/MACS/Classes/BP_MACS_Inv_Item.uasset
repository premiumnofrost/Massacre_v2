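; MACS inventory item actor, shown as a world mesh or as equipment attached to its owner.
; Construction loads item data from DT_MACS_Items by ItemID; OnRep_Item reruns BeginPlay.
; When equipped, it spawns static/skeletal meshes on owner or previously spawned part sockets, using own AnimBP or leader pose, and adds a trace component.
; SetMeshHiddenInGameOnServer toggles parts by socket, e.g. arrows, and updates IsReadyWeapon.
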(event `BeginPlay`
  ;[1 1 1] Set the SM to world when item dropped / Not equipped
  (if (`self.EquippedItem`)
    ;[1 1 1] Hide the World Base Mesh
    (`SceneComponent.SetHiddenInGame` (`self.SM_WorldBase`) true false)
    (for _array_element (`.MeshesToAttach_125_FE5012864988134FDE06A7A5AA085EC3` (break `/Game/MACS/DataModels/S_MACS_Item` (break `/Game/MACS/DataModels/S_MACS_WorldItem` (`self.Item`))))
      ;[1 1 1] Attach each SM or SK on Pawn
      (`|ExecutionSequence`
        (:`then_0`
          (`/Engine/EditorBlueprintResources/StandardMacros.IsValid` (`.StaticMesh_8_8119D24248390B03B983D1B36DD94380` (break `/Game/MACS/DataModels/S_MACS_MeshToAttach` _array_element))
            (:`Is Valid`
              (bind _returnvalue (`|AddComponentByClass` "/Script/Engine.StaticMeshComponent" true))
              (`KismetArrayLibrary.Array_AddUnique` (`self.PrimitiveCompRefs`) _returnvalue)
              (`SceneComponent.SetHiddenInGame` _returnvalue (`.HiddenInGame_28_BC9C2A4246713ECAEEB2728799CD5034` (break `/Game/MACS/DataModels/S_MACS_MeshToAttach` _array_element)) false)
              (`self.AttachToMesh` _returnvalue (`.BoneSocketToAttach_5_08909E59468C9B5FFCF6F8BEA1A3941F` (break `/Game/MACS/DataModels/S_MACS_MeshToAttach` _array_element)))
              (`StaticMeshComponent.SetStaticMesh` _returnvalue (`.StaticMesh_8_8119D24248390B03B983D1B36DD94380` (break `/Game/MACS/DataModels/S_MACS_MeshToAttach` _array_element)))
              (`SceneComponent.SetMobility` _returnvalue "Movable")
              (`PrimitiveComponent.SetCollisionResponseToAllChannels` _returnvalue "ECR_Overlap"))))
        (:`then_1`
          (`/Engine/EditorBlueprintResources/StandardMacros.IsValid` (break `/Game/MACS/DataModels/S_MACS_MeshToAttach` _array_element)
            (:`Is Valid`
              (bind _returnvalue_2 (`|AddComponentByClass` "/Script/Engine.SkeletalMeshComponent" true))
              (`KismetArrayLibrary.Array_AddUnique` (`self.PrimitiveCompRefs`) _returnvalue_2)
              (`SceneComponent.SetHiddenInGame` _returnvalue_2 (`.HiddenInGame_28_BC9C2A4246713ECAEEB2728799CD5034` (break `/Game/MACS/DataModels/S_MACS_MeshToAttach` _array_element)) false)
              (`self.AttachToMesh` _returnvalue_2 (`.BoneSocketToAttach_5_08909E59468C9B5FFCF6F8BEA1A3941F` (break `/Game/MACS/DataModels/S_MACS_MeshToAttach` _array_element)))
              (`SkinnedMeshComponent.SetSkinnedAssetAndUpdate` _returnvalue_2 (break `/Game/MACS/DataModels/S_MACS_MeshToAttach` _array_element) true)
              (`self.SetAnim` _returnvalue_2 (`.SK_AnimInstClass_15_D45710B845526AFAA65544B456D028C1` (break `/Game/MACS/DataModels/S_MACS_MeshToAttach` _array_element)))
              (`SceneComponent.SetMobility` _returnvalue_2 "Movable")
              (`PrimitiveComponent.SetCollisionResponseToAllChannels` _returnvalue_2 "ECR_Overlap")))))
      ;[1 1 1] Add Trace Component at first time
      (`/Engine/EditorBlueprintResources/StandardMacros.IsValid` (`self.GetComponentByClass` "/Game/MACS/Classes/Components/BP_MACS_TraceComp.BP_MACS_TraceComp_C")
        (:`Is Not Valid`
          (`|AddComponentByClass` "/Game/MACS/Classes/Components/BP_MACS_TraceComp.BP_MACS_TraceComp_C"))))
    (else
      (`/Engine/EditorBlueprintResources/ActorMacros.Switch Has Authority`
        (:`Authority`
          (`StaticMeshComponent.SetStaticMesh` (`self.SM_WorldBase`) (`.WorldMesh_124_4D57C2AE48B473BCC9AEB4AD8E30FE0C` (break `/Game/MACS/DataModels/S_MACS_Item` (break `/Game/MACS/DataModels/S_MACS_WorldItem` (`self.Item`))))))))))

(event `SetMeshHiddenInGameOnServer`
  (params (MeshAttachToThisScoket :type Name) (HiddenInGame :type Boolean))
  ;[1 1 1] Set Comp to be Hidden in game like arrows
  (for (_array_element _array_index) (`.MeshesToAttach_125_FE5012864988134FDE06A7A5AA085EC3` (break `/Game/MACS/DataModels/S_MACS_Item` (break `/Game/MACS/DataModels/S_MACS_WorldItem` (`self.Item`))))
    (if (== (`.BoneSocketToAttach_5_08909E59468C9B5FFCF6F8BEA1A3941F` (break `/Game/MACS/DataModels/S_MACS_MeshToAttach` _array_element)) MeshAttachToThisScoket)
      (for (_array_element_2 _array_index_2) (`self.PrimitiveCompRefs`)
        (if (== _array_index_2 _array_index)
          (`SceneComponent.SetHiddenInGame` _array_element_2 HiddenInGame false)
          (set `self.IsReadyWeapon` (not HiddenInGame)))))))

(fn `AttachToMesh`
  (params (MeshAdded :type "PrimitiveComponent Object Reference") (SocketBoneName :type Name))
  (bind _returnvalue (`self.GetComponentByClass` (`self.GetOwner`) "/Script/Engine.SkeletalMeshComponent"))
  (if (`SceneComponent.DoesSocketExist` _returnvalue SocketBoneName)
    (`SceneComponent.K2_AttachToComponent` MeshAdded _returnvalue SocketBoneName "SnapToTarget" "SnapToTarget" "SnapToTarget" true)
    (return)
    (else
      (for _array_element (`self.PrimitiveCompRefs`)
        (`/Engine/EditorBlueprintResources/StandardMacros.IsValid` _array_element
          (:`Is Valid`
            (if (`SceneComponent.DoesSocketExist` _array_element (`local.SocketBoneName`))
              (`SceneComponent.K2_AttachToComponent` (`local.MeshAdded`) _array_element (`local.SocketBoneName`) "SnapToTarget" "SnapToTarget" "SnapToTarget" true)
              (return)))))
      ;[1 1 1] Using own skeletal like Fighter
      (`SceneComponent.K2_AttachToComponent` (`local.MeshAdded`) (`self.GetComponentByClass` (`self.GetOwner`) "/Script/Engine.SkeletalMeshComponent") "None" "SnapToTarget" "SnapToTarget" "SnapToTarget" true)
      (return))))

(fn `OnRep_Item`
  (`self.BeginPlay`))

(fn `SetAnim`
  (params (SK_Element :type "SkeletalMeshComponent Object Reference") (AnimInstClass :type "Object Class Reference"))
  (bind _returnvalue (`self.GetComponentByClass` (`self.GetOwner`) "/Script/Engine.SkeletalMeshComponent"))
  (if (`KismetSystemLibrary.IsValidClass` AnimInstClass)
    (`SkeletalMeshComponent.SetAnimInstanceClass` SK_Element AnimInstClass)
    (`SkeletalMeshComponent.SetAnimationMode` SK_Element "AnimationBlueprint" true)
    (else
      (`SkeletalMeshComponent.SetAnimInstanceClass` SK_Element (`GameplayStatics.GetObjectClass` (`SkeletalMeshComponent.GetAnimInstance` _returnvalue)))
      (`SkinnedMeshComponent.SetLeaderPoseComponent` SK_Element _returnvalue true false))))

(fn `SetWorldCollisions`
  (params (SM_Component :type "StaticMeshComponent Object Reference"))
  (`PrimitiveComponent.SetCollisionResponseToAllChannels` SM_Component "ECR_Ignore")
  (`PrimitiveComponent.SetCollisionResponseToChannel` SM_Component "ECC_WorldStatic" "ECR_Block")
  (`PrimitiveComponent.SetCollisionResponseToChannel` SM_Component "ECC_WorldDynamic" "ECR_Block")
  (`PrimitiveComponent.SetCollisionResponseToChannel` SM_Component "ECC_Pawn" "ECR_Ignore")
  (`PrimitiveComponent.SetMassOverrideInKg` SM_Component "None" 30.0 true)
  (set `PrimitiveComponent.CanCharacterStepUpOn` "ECB_No" SM_Component))

(fn `UserConstructionScript`
  (bind _sm_worldbase (`self.SM_WorldBase`))
  (bind _returnvalue (`KismetStringLibrary.Conv_StringToName` (`KismetStringLibrary.Conv_IntToString` (`self.ItemID`))))
  ;[1 1 1] Construct the Item based on ItemID
  (bind _returnvalue_2 (`DataTableFunctionLibrary.DoesDataTableRowExist` "/Game/MACS/DataModels/DT_MACS_Items.DT_MACS_Items" _returnvalue))
  (if _returnvalue_2
    (bind _returnvalue_3 (`|GetDataTableRow` "/Game/MACS/DataModels/DT_MACS_Items.DT_MACS_Items" _returnvalue)
      (:`then`
        (set `self.Item` (make `/Game/MACS/DataModels/S_MACS_WorldItem` _returnvalue_3 (`self.WorldItemStackAmount`))))
      (:`RowNotFound`
        ;[1 1 1] If ItemID is invalid
        (`StaticMeshComponent.SetStaticMesh` _sm_worldbase null :!label _label)
        (`SceneComponent.SetWorldScale3D` _sm_worldbase (1.0 1.0 1.0))
        (`self.SetWorldCollisions` _sm_worldbase)))
    (else
      (`/Engine/EditorBlueprintResources/ActorMacros.Switch Has Authority`
        (:`Authority`
          (goto _label))))))