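; Base MACS projectile that explodes on hit and damages multiple valid targets within a radius.
; It plays a launch sound at BeginPlay; sphere hits spawn a Niagara effect and, unless the instigator was hit, call MakeExplosionOnServer.
; That event capsule-traces for targets, applies GameplayEffect damage through the owning ability and sends hit reactions.
; With a valid ability, it then plays the impact GameplayCue and sound and destroys itself.
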(event `self.ReceiveBeginPlay`
  ;[1 1 1] SpawnSound At Begin play
  (`GameplayStatics.SpawnSoundAtLocation` (`self.SfxWhenLaunch`) (`self.K2_GetActorLocation`) (struct) 1.0 1.2 0.0 null null))

(event `MakeExplosionOnServer`
  (bind _array (`|MakeArray` (make `/Game/MACS/DataModels/E_MACS_TraceInfo` "NewEnumerator0" "NewEnumerator3" "None" 1.0) :!type "/Game/MACS/DataModels/E_MACS_TraceInfo Structure"))
  ;[1 1 1] When projectile hit, Spawn the PS, make a multi sphere trace looking for target and send this target to ability as gameplay event
  (bind _outhits (`/Game/MACS/Classes/BPL_MACS.MultiCapsuleTraceForActors` self (`self.RadiusToTraceWhenHit`) (`self.ObjectTypesToTraceWhenHit`) (`|MakeArray` (`self.Instigator`) :!type "Actor Object Reference")))
  (for _array_element _outhits
    ;;[1 1 1] Filter the targets
    (if (`/Game/MACS/Classes/BPL_MACS.IsValidTarget` (`self.Instigator`) (`.HitActor` (`GameplayStatics.BreakHitResult` _array_element)))
      ;[1 1 1] Apply GE Damage to target
      (bind _abilityref (`self.AbilityRef`)
        (:`then`
          (bind _returnvalue (`|GenericCreateObject` "/Game/MACS/Classes/BP_MACS_TraceInfo.BP_MACS_TraceInfo_C" _array))
          (`/Game/MACS/Classes/BPL_MACS.Apply GE Damage to Target` _abilityref (`AbilitySystemBlueprintLibrary.AbilityTargetDataFromHitResult` _array_element) (`self.DamageWhenProjectileHit`) _returnvalue)
          ;[1 1 1] Send HitReaction Event
          (message `/Game/MACS/Classes/Interfaces/BPI_MACS_Character.SetHitReaction` (`.HitActor` (`GameplayStatics.BreakHitResult` _array_element)) (make `/Game/MACS/DataModels/S_MACS_HitReaction` self (`|GetArrayItem` _array) _array_element null)))
        (:`else`))))
  (bind _abilityref_2 (`self.AbilityRef`)
    (:`then`
      (`/Game/MACS/Classes/BPL_MACS.Play GC` _abilityref_2 (`self.CueImpact`) (`AbilitySystemBlueprintLibrary.AbilityTargetDataFromHitResult` _array_element))
      (`GameplayStatics.SpawnSoundAtLocation` (`self.SfxWhenHit`) (`self.K2_GetActorLocation`) (struct) 1.0 1.0 0.0 null null)
      (`self.K2_DestroyActor`))
    (:`else`)))

(event `self.Sphere.OnComponentHit`
  (params (HitComponent :type "PrimitiveComponent Object Reference") (OtherActor :type "Actor Object Reference") (OtherComp :type "PrimitiveComponent Object Reference") (NormalImpulse :type "Vector Structure") (Hit :type "HitResult Structure (by ref)"))
  ;[1 1 1] When projectile hit, Spawn the PS, make a multi sphere trace looking for target and send this target to ability as gameplay event
  (`NiagaraFunctionLibrary.SpawnSystemAtLocation` (`self.NsWhenHitSomething`) Hit_Location)
  (if (!= OtherActor (`self.Instigator`))
    (`self.MaKeExplosionOnServer`)))

(fn `UserConstructionScript`)