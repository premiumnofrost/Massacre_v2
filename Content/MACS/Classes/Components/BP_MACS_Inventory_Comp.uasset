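; Pawn inventory component for two weapon slots, handling pickup, replace, toggle, drop and drop-all of BP_MACS_Inv_Item actors.
; GAS gameplay events trigger server calls, most waiting for the UsingAbility tag to clear, that edit the inventory and spawn or destroy item actors.
; The WeaponSlotInUse RepNotify swaps weapon visibility and, on authority, reapplies the weapon's GameplayEffects.
; A looping local sphere trace shows Equip or Replace text on the HUD.
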(event `self.ReceiveBeginPlay`
  (bind _pawnref (`self.PawnRef`))
  (bind _pawnref_2 (`self.PawnRef`))
  ;[1 1 1] Both Sides(Client and Server) execute
  (`|ExecutionSequence`
    (:`then_0`
      (bind _returnvalue (`KismetSystemLibrary.K2_SetTimer` null "SetRef" 0.2 true))
      (set `self.SetRefTimer` _returnvalue))
    (:`then_1`
      (`KismetSystemLibrary.Delay` 0.5)
      (`|ExecutionSequence`
        (:`then_0`
          (`AbilityAsync_WaitGameplayEvent.WaitGameplayEventToActor` _pawnref (struct :`TagName` "MACS_GAS.Abilities.Events.SetWeaponClass.TryToEquip")
            (:`EventReceived`
              (`AbilityAsync_WaitGameplayTagRemoved.WaitGameplayTagRemoveFromActor` _pawnref_2 (struct :`TagName` "MACS_GAS.Abilities.States.UsingAbility") true
                (:`Removed`
                  (`self.CanModifyTheWeapons`)
                  (`self.TryToGetWorldItemOnServer`))))))
        (:`then_1`
          (`AbilityAsync_WaitGameplayEvent.WaitGameplayEventToActor` _pawnref (struct :`TagName` "MACS_GAS.Inventory.Events.SetWeaponClass.ToggleEquippedWeapon")
            (:`EventReceived`
              (`AbilityAsync_WaitGameplayTagRemoved.WaitGameplayTagRemoveFromActor` _pawnref_2 (struct :`TagName` "MACS_GAS.Abilities.States.UsingAbility") true
                (:`Removed`
                  (`self.CanModifyTheWeapons`)
                  (`self.ToogleWeaponSlotInUseOnServer`))))))
        (:`then_2`
          (`AbilityAsync_WaitGameplayEvent.WaitGameplayEventToActor` _pawnref (struct :`TagName` "MACS_GAS.Abilities.Events.SetWeaponClass.TryToDrop")
            (:`EventReceived`
              (`AbilityAsync_WaitGameplayTagRemoved.WaitGameplayTagRemoveFromActor` (`self.PawnRef`) (struct :`TagName` "MACS_GAS.Abilities.States.UsingAbility") true
                (:`Removed`
                  (`self.DropInventoryIndexOnServer`))))))
        (:`then_3`
          (`AbilityAsync_WaitGameplayEvent.WaitGameplayEventToActor` _pawnref (struct :`TagName` "MACS_GAS.Abilities.Events.SetWeaponClass.TryToDropAll")
            (:`EventReceived`
              (`self.DropAllInventoryOnServer`))))
        (:`then_4`
          (`KismetSystemLibrary.K2_SetTimer` null "LocalScanForItems" 0.1 true))))))

(event `TryToGetWorldItemOnServer`
  ;[1 0 0] Server Only
  (bind _hititem (`self.TraceForItems`))
  (`self.TryToGetWorldItem` _hititem))

(event `ToogleWeaponSlotInUseOnServer`
  ;[1 0 0] Server Only
  (`self.ToogleWeaponSlotInUse`))

(event `DropInventoryIndexOnServer`
  ;[1 0 0] Server Only
  (`self.DropInventorySlot` (`self.WeaponSlotInUse`)))

(event `DropAllInventoryOnServer`
  ;[1 0 0] Server Only
  (`self.DropAllInventory`))

(fn `CreateItems`
  (bind _pawnref (`self.PawnRef`))
  ;[1 1 1] Spawn the weapon and store in a variable....the attachment is done inside the BP Inv Item when it is constructed
  (for _array_element (`self.Inventory`)
    (if (`|EnumEquality` (`.Slot_19_ADE0230149EFC7CC090F228AEC686EB6` (break `/Game/MACS/DataModels/S_MACS_InventoryItem` _array_element)) (`self.WeaponSlotInUse`))
      (bind _returnvalue (`|SpawnActorFromClass` "/Game/MACS/Classes/BP_MACS_Inv_Item.BP_MACS_Inv_Item_C" (`Actor.GetTransform` _pawnref) "AlwaysSpawn" "OverrideRootScale" _pawnref (break `/Game/MACS/DataModels/S_MACS_Item` (break `/Game/MACS/DataModels/S_MACS_InventoryItem` _array_element)) 1 true (`Actor.Instigator` _pawnref)))
      (switch `/Game/MACS/DataModels/E_MACS_InventorySlots` (`self.WeaponSlotInUse`)
        (:`NewEnumerator0`
          (set `self.WeaponActor1` _returnvalue))
        (:`NewEnumerator4`
          (set `self.WeaponActor2` _returnvalue))))))

(fn `DropAllInventory`
  (bind _pawnref (`self.PawnRef`))
  ;[1 1 1] For each inventory item
  (for (_array_element _array_index) (`self.Inventory`)
    ;[1 1 1] Spawn the Inv Item in the World
    (`|ExecutionSequence`
      (:`then_0`
        (bind _output (`|GetArrayItem` (`self.Inventory`) _array_index))
        (`|SpawnActorFromClass` "/Game/MACS/Classes/BP_MACS_Inv_Item.BP_MACS_Inv_Item_C" (`KismetMathLibrary.MakeTransform` (+ (`Actor.K2_GetActorLocation` _pawnref) (* (`Actor.GetActorForwardVector` _pawnref) 100.0))) "AlwaysSpawn" "OverrideRootScale" null (break `/Game/MACS/DataModels/S_MACS_Item` (break `/Game/MACS/DataModels/S_MACS_InventoryItem` _output)) (`.StackAmount_20_3F991D074575CDAE34B5918F548EF2E2` (break `/Game/MACS/DataModels/S_MACS_InventoryItem` _output)) false null))
      (:`then_1`
        ;[1 1 1] Destroy the Item's actor storage on variables
        (switch `/Game/MACS/DataModels/E_MACS_InventorySlots` (`.Slot_19_ADE0230149EFC7CC090F228AEC686EB6` (break `/Game/MACS/DataModels/S_MACS_InventoryItem` _array_element))
          (:`NewEnumerator0`
            (`Actor.K2_DestroyActor` (`self.WeaponActor1`)))
          (:`NewEnumerator4`
            (`Actor.K2_DestroyActor` (`self.WeaponActor2`)))))
      (:`then_2`
        ;[1 1 1] Set Weapon Slot in Use as Null
        (set `self.WeaponSlotInUse` "NewEnumerator22"))))
  ;[1 1 1] Clear the Inventory
  (`KismetArrayLibrary.Array_Clear` (`self.Inventory`))
  (return))

(fn `DropInventorySlot`
  (params (InventorySlot :type "/Game/MACS/DataModels/E_MACS_InventorySlots Enum" :default "NewEnumerator22"))
  (bind _pawnref (`self.PawnRef`))
  ;[1 1 1] For each Inventory item
  (for (_array_element _array_index) (`self.Inventory`)
    (if (`|EnumEquality` (`.Slot_19_ADE0230149EFC7CC090F228AEC686EB6` (break `/Game/MACS/DataModels/S_MACS_InventoryItem` _array_element)) InventorySlot)
      (`|ExecutionSequence`
        (:`then_0`
          (bind _output (`|GetArrayItem` (`self.Inventory`) _array_index))
          ;[1 1 1] Spawn Item on world
          (`|SpawnActorFromClass` "/Game/MACS/Classes/BP_MACS_Inv_Item.BP_MACS_Inv_Item_C" (`KismetMathLibrary.MakeTransform` (+ (`Actor.K2_GetActorLocation` _pawnref) (* (`Actor.GetActorForwardVector` _pawnref) 100.0))) "AlwaysSpawn" "OverrideRootScale" null (break `/Game/MACS/DataModels/S_MACS_Item` (break `/Game/MACS/DataModels/S_MACS_InventoryItem` _output)) (`.StackAmount_20_3F991D074575CDAE34B5918F548EF2E2` (break `/Game/MACS/DataModels/S_MACS_InventoryItem` _output)) false null))
        (:`then_1`
          ;[1 1 1] Remove Item from inventory
          (`KismetArrayLibrary.Array_Remove` (`self.Inventory`) _array_index))
        (:`then_2`
          ;[1 1 1] Change the WeaponClass in Use
          (switch `/Game/MACS/DataModels/E_MACS_InventorySlots` (`local.InventorySlot`)
            (:`NewEnumerator0`
              (`Actor.K2_DestroyActor` (`self.WeaponActor1`))
              (set `self.WeaponSlotInUse` "NewEnumerator4"))
            (:`NewEnumerator4`
              (`Actor.K2_DestroyActor` (`self.WeaponActor2`))
              (set `self.WeaponSlotInUse` "NewEnumerator0"))))
        (:`then_3`
          (return))))))

(fn `GetAllActorsFromClass`
  (params (ActorClass :type "Actor Class Reference"))
  (returns (OutActors :type "Array of Actor Object Reference"))
  (locals (LocalArray :type "Array of Actor Object Reference"))
  (bind _outactors (`GameplayStatics.GetAllActorsOfClass` ActorClass))
  (return _outactors))

(fn `GetCurrentWeaponActor`
  (returns (WeaponInUse :type "/Game/MACS/Classes/BP_MACS_Inv_Item Object Reference"))
  (return (cast `/Game/MACS/Classes/BP_MACS_Inv_Item` (select `/Game/MACS/DataModels/E_MACS_InventorySlots` (`self.WeaponSlotInUse`) :`NewEnumerator0` (`self.WeaponActor1`) :`NewEnumerator4` (`self.WeaponActor2`)) :!pure true)))

(fn `GetFreeWeaponSlot`
  (returns (WeaponsCount :type "/Game/MACS/DataModels/E_MACS_InventorySlots Enum"))
  (locals (FreeWeaponSlot :type "/Game/MACS/DataModels/E_MACS_InventorySlots Enum"))
  ;[1 1 1] Get the Free weapon slot if have one or return null
  (set `local.FreeWeaponSlot` "NewEnumerator0")
  (for _array_element (`self.Inventory`)
    (if (`|EnumEquality` (`.Slot_19_ADE0230149EFC7CC090F228AEC686EB6` (break `/Game/MACS/DataModels/S_MACS_InventoryItem` _array_element)) "NewEnumerator0")
      (set `local.FreeWeaponSlot` "NewEnumerator4")
      (for _array_element_2 (`self.Inventory`)
        (if (`|EnumEquality` (`.Slot_19_ADE0230149EFC7CC090F228AEC686EB6` (break `/Game/MACS/DataModels/S_MACS_InventoryItem` _array_element_2)) "NewEnumerator4")
          (set `local.FreeWeaponSlot` "NewEnumerator22")))
      (return (`local.FreeWeaponSlot`))))
  (return (`local.FreeWeaponSlot`)))

(fn `GetItemBySlot`
  (params (Slot :type "/Game/MACS/DataModels/E_MACS_InventorySlots Enum" :default "NewEnumerator22"))
  (returns (Item :type "/Game/MACS/DataModels/S_MACS_Item Structure"))
  ;[1 1 1] The the Item on inventory by passing the Slot
  (for _array_element (`self.Inventory`)
    (if (`|EnumEquality` (`.Slot_19_ADE0230149EFC7CC090F228AEC686EB6` (break `/Game/MACS/DataModels/S_MACS_InventoryItem` _array_element)) Slot)
      (return (break `/Game/MACS/DataModels/S_MACS_InventoryItem` _array_element))))
  (return (make `/Game/MACS/DataModels/S_MACS_Item` :`WorldMesh` null :`Icon` null)))

(fn `LocalScanForItems`
  (bind (_item_id _item_name) (break `/Game/MACS/DataModels/S_MACS_Item` (`self.GetItemBySlot` (`self.WeaponSlotInUse`))))
  ;[1 1 1] Local trace for Inv Items in the world to show the Item Name on widget
  (bind _pawnref (`self.PawnRef`)
    (:`then`
      (bind _asplayer_controller (cast `PlayerController` (`Pawn.GetController` (`Actor.Instigator` _pawnref))))
      (bind _asbp_macs_hud (cast `/Game/MACS/UI/BP_MACS_HUD` (`PlayerController.GetHUD` _asplayer_controller)))
      (bind _hititem (`self.TraceForItems`))
      (bind _asbp_macs_inv_item (cast `/Game/MACS/Classes/BP_MACS_Inv_Item` _hititem)
        (:`then`
          (if (`|EnumEquality` (`self.GetFreeWeaponSlot`) "NewEnumerator22")
            (bind _returnvalue (`KismetStringLibrary.Conv_NameToString` (`.Name_83_E527BB6041CE9327AFFD8D8FA3C7D0D3` (break `/Game/MACS/DataModels/S_MACS_Item` (break `/Game/MACS/DataModels/S_MACS_WorldItem` (`/Game/MACS/Classes/BP_MACS_Inv_Item.Item` _asbp_macs_inv_item))))))
            (bind _bp_macs_gas_actiontext (`/Game/MACS/UI/WB_MACS_UI.BP_MACS_GAS_ActionText` (`/Game/MACS/UI/BP_MACS_HUD.UI` _asbp_macs_hud)))
            (set `/Game/MACS/UI/WB_MACS_ActionText.ActionText` (`KismetTextLibrary.Conv_StringToText` (`KismetStringLibrary.Concat_StrStr` "Replace " (`KismetStringLibrary.Conv_NameToString` _item_name) " for " _returnvalue)) _bp_macs_gas_actiontext)
            (else
              (set `/Game/MACS/UI/WB_MACS_ActionText.ActionText` (`KismetTextLibrary.Conv_StringToText` (`KismetStringLibrary.Concat_StrStr` "Equip " _returnvalue)) _bp_macs_gas_actiontext))))
        (:`CastFailed`
          (set `/Game/MACS/UI/WB_MACS_ActionText.ActionText` "" _bp_macs_gas_actiontext))))
    (:`else`)))

(fn `OnRep_WeaponSlotInUse`
  ;[1 1 1] Run on all when the Weapon Slot in Use change value
  (`self.UpdateWeaponSlotInUse`)
  ;[1 1 1] Server Only
  (`/Engine/EditorBlueprintResources/ActorComponentMacros.Switch Has Authority`
    (:`Authority`
      (`self.UpdateItemGE`))))

(fn `SetRef`
  (bind _returnvalue (`self.GetOwner`))
  (`|ExecutionSequence`
    (:`then_0`
      (`/Engine/EditorBlueprintResources/StandardMacros.IsValid` _returnvalue
        (:`Is Valid`
          (set `self.PawnRef` _returnvalue)
          (`KismetSystemLibrary.K2_ClearAndInvalidateTimerHandle` (`self.SetRefTimer`))
          (return))))))

(fn `ToogleWeaponSlotInUse`
  ;[1 1 1] Set w/ notify the Weapon slot in use to show or hide the meshes on pawn
  (if (`|EnumEquality` (`self.GetFreeWeaponSlot`) "NewEnumerator22")
    (switch `/Game/MACS/DataModels/E_MACS_InventorySlots` (`self.WeaponSlotInUse`)
      (:`NewEnumerator0`
        (set `self.WeaponSlotInUse` "NewEnumerator4"))
      (:`NewEnumerator4`
        (set `self.WeaponSlotInUse` "NewEnumerator0")))))

(fn `TraceForItems`
  (returns (HitItem :type "Actor Object Reference"))
  (locals (ActorsToIgnore :type "Array of Actor Object Reference") (LocalTrace :type "EDrawDebugTrace Enum" :default "ForOneFrame"))
  (bind _actorstoignore (`local.ActorsToIgnore`))
  (bind _returnvalue (`SceneComponent.K2_GetComponentLocation` (`Actor.GetComponentByClass` (`self.PawnRef`) "/Script/Engine.SkeletalMeshComponent")))
  (`self.PawnRef`
    (:`then`
      ;[1 1 1] Get All actor to ignore
      (`KismetArrayLibrary.Array_Append` _actorstoignore (`self.GetAllActorsFromClass` "/Game/MACS/Demo/DemoRoom/Blueprints/BP_DemoRoom.BP_DemoRoom_C"))
      (`KismetArrayLibrary.Array_Append` _actorstoignore (`self.GetAllActorsFromClass` "/Game/MACS/Classes/BP_MACS_Character_Base.BP_MACS_Character_Base_C"))
      (`KismetArrayLibrary.Array_Append` _actorstoignore (`self.GetAllActorsFromClass` "/Script/Engine.TriggerBase"))
      ;[1 1 1] Trace For Inv Item
      (bind _debugtrace (message `/Game/MACS/Classes/Interfaces/BPI_MACS_Character.GetDebugTrace` (`self.PawnRef`)))
      (bind (_outhits _returnvalue_2) (`KismetSystemLibrary.SphereTraceMultiForObjects` _returnvalue _returnvalue (`self.TraceRadiusForItems`) (`|MakeArray` "ObjectTypeQuery2" :!type "EObjectTypeQuery Enum") true (`local.ActorsToIgnore`) (select `bool` _debugtrace :`true` "ForOneFrame" :!type "EDrawDebugTrace Enum") true (struct :`R` 1.0 :`A` 1.0) (struct :`G` 1.0 :`A` 1.0) 3.0))
      (if _returnvalue_2
        (for _array_element _outhits
          (bind _asbp_macs_inv_item (cast `/Game/MACS/Classes/BP_MACS_Inv_Item` (`.HitActor` (`GameplayStatics.BreakHitResult` _array_element))))
          ;;[1 1 1] Don't trace equipped items
          (if (not (`/Game/MACS/Classes/BP_MACS_Inv_Item.EquippedItem` _asbp_macs_inv_item))
            (return _asbp_macs_inv_item)))))
    (:`else`)))

(fn `TryToGetWorldItem`
  (params (HitItem :type "Actor Object Reference"))
  (locals (InvWorldItem :type "/Game/MACS/Classes/BP_MACS_Inv_Item Object Reference") (CurrentArrayIndexLoop :type Integer))
  (bind _inventory (`self.Inventory`))
  (bind _weaponslotinuse (`self.WeaponSlotInUse`))
  (bind (_item_item _item_stackamount) (break `/Game/MACS/DataModels/S_MACS_WorldItem` (`/Game/MACS/Classes/BP_MACS_Inv_Item.Item` (`local.InvWorldItem`))))
  (bind _asbp_macs_inv_item (cast `/Game/MACS/Classes/BP_MACS_Inv_Item` HitItem))
  (set `local.InvWorldItem` _asbp_macs_inv_item)
  (bind _invworlditem (`local.InvWorldItem`)
    (:`then`
      (switch `/Game/MACS/DataModels/E_MACS_ItemType` (`.ItemType_96_76D9873E45C5C7DF6AEB50B150BFF742` (break `/Game/MACS/DataModels/S_MACS_Item` (break `/Game/MACS/DataModels/S_MACS_WorldItem` (`/Game/MACS/Classes/BP_MACS_Inv_Item.Item` _invworlditem))))
        (:`NewEnumerator0`
          ;[1 1 1] Handle Weapons item type...Other inventory items can be implemented here too
          (switch `/Game/MACS/DataModels/E_MACS_InventorySlots` (`self.GetFreeWeaponSlot`)
            (:`NewEnumerator22`
              (for _array_element (`self.Inventory`)
                (if (`|EnumEquality` (`.Slot_19_ADE0230149EFC7CC090F228AEC686EB6` (break `/Game/MACS/DataModels/S_MACS_InventoryItem` _array_element)) _weaponslotinuse)
                  (`self.DropInventorySlot` _weaponslotinuse)
                  (`self.TryToGetWorldItem` (`local.InvWorldItem`))
                  (return))))
            (:`NewEnumerator0`
              (bind _returnvalue (`KismetArrayLibrary.Array_AddUnique` _inventory (make `/Game/MACS/DataModels/S_MACS_InventoryItem` _item_item _item_stackamount (`self.GetFreeWeaponSlot`)) :!label _label))
              (bind (_output_item _output_stackamount _output_slot) (break `/Game/MACS/DataModels/S_MACS_InventoryItem` (`|GetArrayItem` _inventory _returnvalue)))
              (set `self.WeaponSlotInUse` _output_slot)
              (`Actor.K2_DestroyActor` (`local.InvWorldItem`))
              (`self.CreateItems`)
              (return))
            (:`NewEnumerator4`
              (goto _label))))))
    (:`else`)))

(fn `UpdateItemGE`
  (bind _returnvalue (`AbilitySystemBlueprintLibrary.GetAbilitySystemComponent` (`self.PawnRef`)))
  (bind (_id _name _worldmesh _meshestoattach _icon _weight _itemtype _gameplayeffecttoselfapply) (break `/Game/MACS/DataModels/S_MACS_Item` (`self.GetItemBySlot` (`self.WeaponSlotInUse`))))
  (if (`KismetArrayLibrary.Array_IsNotEmpty` _gameplayeffecttoselfapply)
    (for _array_element _gameplayeffecttoselfapply
      (`/Engine/EditorBlueprintResources/StandardMacros.IsValid` _returnvalue
        (:`Is Valid`
          ;[1 1 1] Select the Classes that you need to be removed before apply a new weaponclass. All TAGs from the items
          (`AbilitySystemComponent.RemoveActiveEffectsWithTags` _returnvalue (`/Game/MACS/Classes/BPL_MACS.GetAllWeaponClassTAGs`))
          ;[1 1 1] Apply the new Gameplay TAG of WeaponClass
          (`AbilitySystemComponent.BP_ApplyGameplayEffectToSelf` :`self` _returnvalue :`GameplayEffectClass` _array_element :`Level` 1.0))))
    (else
      (`AbilitySystemComponent.RemoveActiveEffectsWithTags` _returnvalue (`/Game/MACS/Classes/BPL_MACS.GetAllWeaponClassTAGs`)))))

(fn `UpdateWeaponSlotInUse`
  (bind _weaponactor1 (`self.WeaponActor1`))
  (bind _weaponactor2 (`self.WeaponActor2`))
  (bind _weaponactor2_2 (`self.WeaponActor2`))
  (bind _weaponactor1_2 (`self.WeaponActor1`))
  ;[1 1 1] Show or hide the weapon in use...Use this place to handle the visual swap of weapons like equipe and unequip animations
  (switch `/Game/MACS/DataModels/E_MACS_InventorySlots` (`self.WeaponSlotInUse`)
    (:`NewEnumerator0`
      (`|ExecutionSequence`
        (:`then_0`
          (`/Engine/EditorBlueprintResources/StandardMacros.IsValid` _weaponactor1_2
            (:`Is Valid`
              (`Actor.SetActorHiddenInGame` _weaponactor1_2 false))))
        (:`then_1`
          (`/Engine/EditorBlueprintResources/StandardMacros.IsValid` _weaponactor2
            (:`Is Valid`
              (`Actor.SetActorHiddenInGame` _weaponactor2 true))))))
    (:`NewEnumerator4`
      (`|ExecutionSequence`
        (:`then_0`
          (`/Engine/EditorBlueprintResources/StandardMacros.IsValid` _weaponactor2_2
            (:`Is Valid`
              (`Actor.SetActorHiddenInGame` _weaponactor2_2 false))))
        (:`then_1`
          (`/Engine/EditorBlueprintResources/StandardMacros.IsValid` _weaponactor1
            (:`Is Valid`
              (`Actor.SetActorHiddenInGame` _weaponactor1 true))))))))