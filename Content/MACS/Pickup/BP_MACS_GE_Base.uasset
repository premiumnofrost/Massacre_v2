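; Base pickup pad actor with a floating, spinning mesh that sends a gameplay tag event to an overlapping player character to show action text.
; A server event toggles the cooldown state for a set delay, and its RepNotify hides or restores the mesh and audio, recolors the Niagara effect and spawns pickup bursts.
; The construction script tints the mesh's dynamic material and the Niagara system with a configurable base color.
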(event `self.ReceiveBeginPlay`
  (bind _staticmesh (`self.StaticMesh`))
  (bind (_returnvalue_roll _returnvalue_pitch _returnvalue_yaw) (`KismetMathLibrary.BreakRotator` (`SceneComponent.K2_GetComponentRotation` _staticmesh)))
  (bind (_returnvalue_x _returnvalue_y _returnvalue_z) (`KismetMathLibrary.BreakVector` (`SceneComponent.K2_GetComponentLocation` _staticmesh)))
  ;[1 1 1] Set rotation and location of floating mesh
  (bind (_direction _curve) (`Timeline|FloatingMeshTimeline` :!via `PlayFromStart`)
    (:`Update`
      (`SceneComponent.K2_SetWorldLocationAndRotation` _staticmesh (`KismetMathLibrary.MakeVector` _returnvalue_x _returnvalue_y (+ _returnvalue_z _curve)) (`KismetMathLibrary.MakeRotator` _returnvalue_roll _returnvalue_pitch (+ _returnvalue_yaw 1.0)) false false))))

(event `self.Capsule.OnComponentBeginOverlap`
  (params (OverlappedComponent :type "PrimitiveComponent Object Reference") (OtherActor :type "Actor Object Reference") (OtherComp :type "PrimitiveComponent Object Reference") (OtherBodyIndex :type Integer) (bFromSweep :type Boolean) (SweepResult :type "HitResult Structure (by ref)"))
  (bind _gameplaytagoverlapsomething (`self.GameplayTagOverlapSomething`))
  ;[1 1 1] Send gameplay event to player who overlap this actor to show action text
  (bind _ascharacter (cast `Character` OtherActor))
  (if (`Pawn.IsPlayerControlled` _ascharacter)
    (`AbilitySystemBlueprintLibrary.SendGameplayEventToActor` OtherActor _gameplaytagoverlapsomething (make `GameplayEventData` _gameplaytagoverlapsomething null self null null (struct) (struct) (`BlueprintGameplayTagLibrary.MakeGameplayTagContainerFromArray` (`|MakeArray` (`self.GameplayTagOverlapSomethingBegin`)))))))

(event `SetPickupCooldownOnServer`
  ;[1 1 1] Set pickup cooldown on server and repnotify
  (set `self.CooldownState` true)
  (`KismetSystemLibrary.Delay` (`self.Cooldown`))
  (set `self.CooldownState` false))

(fn `OnRep_Active`
  (bind _returnvalue (`self.K2_GetActorLocation`))
  (bind _ns (`self.NS`))
  (bind _colortochange_basecolor (`self.ColorToChange_BaseColor`))
  (bind _staticmesh (`self.StaticMesh`))
  (bind _niagaraparametertochangecolor (`self.NiagaraParameterToChangeColor`))
  (bind _audio (`self.Audio`))
  (bind _niagaraparametertochangecolor_2 (`self.NiagaraParameterToChangeColor`))
  (if (`self.CooldownState`)
    (`FXSystemComponent.SetColorParameter` _ns _niagaraparametertochangecolor_2 (struct :`G` 1.0))
    (`SceneComponent.SetVisibility` _staticmesh false false)
    (`ActorComponent.SetActive` _audio false false)
    (bind _returnvalue_2 (`NiagaraFunctionLibrary.SpawnSystemAtLocation` (`self.NsWhenPickup2`) _returnvalue))
    (`/Engine/EditorBlueprintResources/StandardMacros.IsValid` _returnvalue_2
      (:`Is Valid`
        (`FXSystemComponent.SetColorParameter` _returnvalue_2 _niagaraparametertochangecolor _colortochange_basecolor)
        (bind _returnvalue_3 (`NiagaraFunctionLibrary.SpawnSystemAtLocation` (`self.NsWhenPickup1`) _returnvalue))
        (`/Engine/EditorBlueprintResources/StandardMacros.IsValid` _returnvalue_3
          (:`Is Valid`
            (`FXSystemComponent.SetColorParameter` _returnvalue_3 _niagaraparametertochangecolor _colortochange_basecolor)))))
    (else
      (`FXSystemComponent.SetColorParameter` _ns _niagaraparametertochangecolor_2 (`self.ColorToChange_BaseColor`))
      (`SceneComponent.SetVisibility` _staticmesh true false)
      (`ActorComponent.SetActive` _audio true false))))

(fn `SetNiagaraBaseColor`
  (bind _mesh (`self.Mesh`))
  (bind _returnvalue (`PrimitiveComponent.CreateDynamicMaterialInstance` _mesh 0 (`PrimitiveComponent.GetMaterial` _mesh 0) "None"))
  (`MaterialInstanceDynamic.SetVectorParameterValue` _returnvalue (`self.ColorToChangeInPickupMesh`) (`self.ColorToChange_BaseColor`))
  (`PrimitiveComponent.SetMaterial` (`self.Mesh`) 0 _returnvalue)
  (`NiagaraComponent.SetVariableLinearColor` (`self.NS`) "GunPad_Color" (`self.ColorToChange_BaseColor`)))

(fn `UserConstructionScript`
  (`self.SetNiagaraBaseColor`))