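; Ghost trail afterimage actor that freezes its instigator's current pose as a fading translucent copy, then destroys itself.
; On BeginPlay it copies the instigator's skeletal mesh and pose into a poseable mesh and spawns a ghost trail Niagara system attached to the instigator's mesh.
; Every material slot gets a dynamic ghost material instance, whose Opacity a timeline drives until it finishes and the actor is destroyed.
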(event `self.ReceiveBeginPlay`
  (bind _poseablemesh (`self.PoseableMesh`))
  (bind _poseablemesh_2 (`self.PoseableMesh`))
  (bind _returnvalue (`self.GetComponentByClass` (`self.Instigator`) "/Script/Engine.SkeletalMeshComponent"))
  (bind (_returnvalue_location _returnvalue_rotation) (`KismetMathLibrary.BreakTransform` (`SceneComponent.K2_GetComponentToWorld` _returnvalue)))
  (`|ExecutionSequence`
    (:`then_0`
      (`SkinnedMeshComponent.SetSkinnedAssetAndUpdate` _poseablemesh (`SkeletalMeshComponent.GetSkeletalMeshAsset` _returnvalue) false)
      (`PoseableMeshComponent.CopyPoseFromSkeletalComponent` _poseablemesh _returnvalue)
      (`NiagaraFunctionLibrary.SpawnSystemAttached` "/Game/MACS/VFX/NS_MACS_GhostTrail.NS_MACS_GhostTrail" _returnvalue "None" _returnvalue_location _returnvalue_rotation "KeepRelativeOffset" true))
    (:`then_1`
      (for (_ _array_index) (`MeshComponent.GetMaterials` _poseablemesh_2)
        (bind _returnvalue_2 (`KismetMaterialLibrary.CreateDynamicMaterialInstance` "/Game/MACS/VFX/MI_MACS_GhostTrail.MI_MACS_GhostTrail"))
        (`KismetArrayLibrary.Array_Add` (`self.DynamicMaterials`) _returnvalue_2)
        (`PrimitiveComponent.SetMaterial` _poseablemesh_2 _array_index _returnvalue_2)))
    (:`then_2`
      (bind (_direction _opacity) (`Timeline|Opacity` :!via `PlayFromStart`)
        (:`Update`
          (for _array_element (`self.DynamicMaterials`)
            (`MaterialInstanceDynamic.SetScalarParameterValue` _array_element "Opacity" _opacity)))
        (:`Finished`
          (`self.K2_DestroyActor`))))))

(fn `UserConstructionScript`)