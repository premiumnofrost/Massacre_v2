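; Base MADS game mode that keeps a persistent global leaderboard and chooses the "Menu"-tagged PlayerStart for players.
; Scores load from a SaveGame slot on BeginPlay and are copied to each BP_MACS_PC at login.
; Score updates replace or add entries by ID, run a swap sort on kills minus half deaths, then push to all controllers and save.
; Logout hands the exiting controller to BPMADSComp for removal.
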(event `self.ReceiveBeginPlay`
  ;[0.03529 0 1] Global Score System
  (`self.LoadGlobalScore`))

(event `self.K2_PostLogin`
  (params (NewPlayer :type "PlayerController Object Reference"))
  ;[0.03529 0 1] Global Score System
  (`self.GetGlobalScorePlayers` NewPlayer))

(event `SetGlobalScoreOnAllClients`
  ;[0.03529 0 1] Global Score System
  (`self.SortGlobalScoreArray` (`self.GlobalScorePlayers`))
  (bind _outactors (`GameplayStatics.GetAllActorsOfClass` "/Game/MACS/Classes/BP_MACS_PC.BP_MACS_PC_C"))
  (for _array_element _outactors
    (set `/Game/MACS/Classes/BP_MACS_PC.Global Score Players` (`self.GlobalScorePlayers`) _array_element)
    (`self.SaveGlobalScore`)))

(event `self.K2_OnLogout`
  (params (ExitingController :type "Controller Object Reference"))
  ;[1 1 1] Login Client
  (`/Game/MADS/Base/BP_MADS_Comp.RemovePlayerAfterLogout` (`self.BP_MADS_Comp`) (make `/Game/MADS/DataModels/S_MADS_ConnectedAccount` (struct :`ID` -1) (cast `PlayerController` ExitingController :!pure true))))

(fn `AddGlobalScorePlayer`
  (params (PlayerScore :type "/Game/MADS/DataModels/S_MADS_CharacterGlobalScore Structure"))
  (locals (PlayerScoreLocal :type "/Game/MADS/DataModels/S_MADS_CharacterGlobalScore Structure"))
  (bind _globalscoreplayers (`self.GlobalScorePlayers`))
  (bind _output_get (set `local.PlayerScoreLocal` PlayerScore))
  (bind _found (`self.FindScorePlayer` _output_get))
  (if _found
    (bind (_found_2 _array_index) (`self.FindScorePlayer` (`local.PlayerScoreLocal`)))
    (`KismetArrayLibrary.Array_Set` _globalscoreplayers _array_index (`local.PlayerScoreLocal`))
    (else
      (`KismetArrayLibrary.Array_AddUnique` _globalscoreplayers (`local.PlayerScoreLocal`))))
  (`self.SetGlobalScoreOnAllClients`)
  (`self.SaveGlobalScore`))

(fn `ChoosePlayerStart`
  (params (Player :type "Controller Object Reference"))
  (returns (ReturnValue :type "Actor Object Reference"))
  (return (`self.GetPlayerStartByTAG` "Menu")))

(fn `FindScorePlayer`
  (params (NewLocalVar1 :type "/Game/MADS/DataModels/S_MADS_CharacterGlobalScore Structure"))
  (returns (Found :type Boolean) (`Array Index` :type Integer))
  (locals (NewLocalVar :type "/Game/MADS/DataModels/S_MADS_CharacterGlobalScore Structure"))
  (for (_array_element _array_index) (`self.GlobalScorePlayers`)
    (bind _returnvalue (== NewLocalVar1_ID_4_F53A75C74278F51E27CB78ACB53485A9 (break `/Game/MADS/DataModels/S_MADS_CharacterGlobalScore` _array_element)))
    (if _returnvalue
      (break)))
  (return _returnvalue _array_index))

(fn `GetGlobalScorePlayers`
  (params (`Player Controller` :type "PlayerController Object Reference"))
  (bind _asbp_macs_pc (cast `/Game/MACS/Classes/BP_MACS_PC` `Player Controller`))
  (set `/Game/MACS/Classes/BP_MACS_PC.Global Score Players` (`self.GlobalScorePlayers`) _asbp_macs_pc)
  (return))

(fn `GetPlayerStartByTAG`
  (params (PlayerStartTAG :type Name))
  (returns (PlayerSpot :type "PlayerStart Object Reference"))
  ;[1 1 1] Return the player start ref with the TAG
  (bind _outactors (`GameplayStatics.GetAllActorsOfClass` "/Script/Engine.PlayerStart"))
  (for _array_element _outactors
    (if (== (`PlayerStart.PlayerStartTag` _array_element) (`local.PlayerStartTAG`))
      (return _array_element))))

(fn `GetScore`
  (params (Kills :type Integer) (Deads :type Integer))
  (returns (Score :type Integer))
  (return (- Kills (* Deads 0.5))))

(fn `LoadGlobalScore`
  (bind _returnvalue (`GameplayStatics.DoesSaveGameExist` "MADS_GlobalScore"))
  (if (not _returnvalue)
    (bind _returnvalue_2 (`GameplayStatics.CreateSaveGameObject` "/Game/MADS/DataModels/SG_MADS_ScoreData.SG_MADS_ScoreData_C"))
    (`GameplayStatics.SaveGameToSlot` _returnvalue_2 "MADS_GlobalScore"))
  (bind _returnvalue_3 (`GameplayStatics.LoadGameFromSlot` "MADS_GlobalScore"))
  (bind _assg_mads_score_data (cast `/Game/MADS/DataModels/SG_MADS_ScoreData` _returnvalue_3))
  (set `self.GlobalScorePlayers` (`/Game/MADS/DataModels/SG_MADS_ScoreData.GlobalScoreData` _assg_mads_score_data)))

(fn `SaveGlobalScore`
  (bind _returnvalue (`GameplayStatics.DoesSaveGameExist` "MADS_GlobalScore"))
  (if _returnvalue
    (bind _returnvalue_2 (`GameplayStatics.CreateSaveGameObject` "/Game/MADS/DataModels/SG_MADS_ScoreData.SG_MADS_ScoreData_C"))
    (set `/Game/MADS/DataModels/SG_MADS_ScoreData.GlobalScoreData` (`self.GlobalScorePlayers`) _returnvalue_2)
    (`GameplayStatics.SaveGameToSlot` _returnvalue_2 "MADS_GlobalScore")
    (else
      (bind _returnvalue_3 (`GameplayStatics.CreateSaveGameObject` "/Game/MADS/DataModels/SG_MADS_ScoreData.SG_MADS_ScoreData_C"))
      (`GameplayStatics.SaveGameToSlot` _returnvalue_3 "MADS_GlobalScore"))))

(fn `SortGlobalScoreArray`
  (params (GlobalScorePlayers :type "Array of /Game/MADS/DataModels/S_MADS_CharacterGlobalScore Structure"))
  (locals (LocalArrayGSP :type "Array of /Game/MADS/DataModels/S_MADS_CharacterGlobalScore Structure"))
  (bind _output_get (set `local.LocalArrayGSP` GlobalScorePlayers))
  (for (_ _array_index) _output_get
    (for (_array_element _array_index_2) (`local.LocalArrayGSP`)
      (bind _output (`|GetArrayItem` (`local.LocalArrayGSP`) _array_index))
      (if (< (`self.GetScore` (break `/Game/MADS/DataModels/S_MADS_CharacterScore` (`.Score_39_528F5DDF42328B0FB63EB9BA7E822FEB` (break `/Game/MADS/DataModels/S_MADS_CharacterGlobalScore` _output))) (`.Deaths_42_B6E7C60B468A0303E82F7A9A572E878F` (break `/Game/MADS/DataModels/S_MADS_CharacterScore` (`.Score_39_528F5DDF42328B0FB63EB9BA7E822FEB` (break `/Game/MADS/DataModels/S_MADS_CharacterGlobalScore` _output))))) (`self.GetScore` (break `/Game/MADS/DataModels/S_MADS_CharacterScore` (`.Score_39_528F5DDF42328B0FB63EB9BA7E822FEB` (break `/Game/MADS/DataModels/S_MADS_CharacterGlobalScore` _array_element))) (`.Deaths_42_B6E7C60B468A0303E82F7A9A572E878F` (break `/Game/MADS/DataModels/S_MADS_CharacterScore` (`.Score_39_528F5DDF42328B0FB63EB9BA7E822FEB` (break `/Game/MADS/DataModels/S_MADS_CharacterGlobalScore` _array_element))))))
        (`KismetArrayLibrary.Array_Swap` (`local.LocalArrayGSP`) _array_index _array_index_2)
        (break)))))

(fn `UserConstructionScript`)