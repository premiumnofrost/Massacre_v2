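; Character preview actor whose scene capture component shows only the actor itself, for render-to-texture display in what appears to be character selection or creation.
; Every tick it reapplies the skeletal mesh from CharData.PersonToPlay with the ABP_MACS anim class.
; Start, move and end rotation functions let mouse drags yaw the mesh, which eases back to zero rotation when released.
; Gender mesh and color tint functions exist but are never run in CustomChar.
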(event `self.ReceiveBeginPlay`
  (`SceneCaptureComponent.ShowOnlyActorComponents` (`self.SceneTo2D_SelectionCreation`) self false))

(event `self.ReceiveTick`
  (params (DeltaSeconds :type "Float (single-precision)"))
  (`self.RestoreToRotation` DeltaSeconds)
  (`self.CustomChar`))

(fn `CustomChar`
  (`self.SetMeshCharacter`))

(fn `EndRotation`
  (set `self.EnableRotation` false))

(fn `MouseRotation`
  (params (MouseRotation :type "Vector2D Structure"))
  (bind _returnvalue_x (`KismetMathLibrary.BreakVector2D` (- MouseRotation (`self.StartMouseRotation`))))
  (if (`self.EnableRotation`)
    (`SceneComponent.K2_AddWorldRotation` (`self.Mesh`) (`KismetMathLibrary.MakeRotator` 0.0 0.0 (* _returnvalue_x -1.0)) false false)
    (set `self.StartMouseRotation` (`local.MouseRotation`))))

(fn `RestoreToRotation`
  (params (Alpha :type "Float (double-precision)"))
  (bind _mesh (`self.Mesh`))
  (if (not (`self.EnableRotation`))
    (`SceneComponent.K2_SetWorldRotation` _mesh (`|EaseFunction` "EaseOut" Alpha (`SceneComponent.K2_GetComponentRotation` _mesh)) false false)))

(fn `SetMeshCharacter`
  (bind (_chardata_id _chardata_owneraccountid _chardata_name _chardata_gender _chardata_color _chardata_level _chardata_transform _chardata_persontoplay) (break `/Game/MADS/DataModels/S_MADS_Character` (`self.CharData`)))
  ;[1 1 1] Set skeletal mesh and textures by gender
  (`SkinnedMeshComponent.SetSkinnedAssetAndUpdate` (`self.Mesh`) _chardata_persontoplay true)
  (`SkeletalMeshComponent.SetAnimInstanceClass` (`self.Mesh`) "/Game/MACS/Animations/ABP_MACS.ABP_MACS_C")
  (`SkeletalMeshComponent.SetAnimInstanceClass` (`self.Mesh`) "/Game/MACS/Animations/ABP_MACS.ABP_MACS_C"))

(fn `SetMeshColor`
  (bind (_chardata_id _chardata_owneraccountid _chardata_name _chardata_gender _chardata_color) (break `/Game/MADS/DataModels/S_MADS_Character` (`self.CharData`)))
  (bind _mesh (`self.Mesh`))
  (for (_array_element _array_index) (`MeshComponent.GetMaterials` _mesh)
    (bind _returnvalue (`PrimitiveComponent.CreateDynamicMaterialInstance` _mesh _array_index _array_element "None"))
    (`MaterialInstanceDynamic.SetVectorParameterValue` _returnvalue "Tint" _chardata_color)))

(fn `SetMeshGender`
  (bind _mesh (`self.Mesh`))
  (bind (_chardata_id _chardata_owneraccountid _chardata_name _chardata_gender) (break `/Game/MADS/DataModels/S_MADS_Character` (`self.CharData`)))
  ;[1 1 1] Set skeletal mesh and textures by gender
  (`SkinnedMeshComponent.SetSkinnedAssetAndUpdate` _mesh (select `int` _chardata_gender :`0` "/Game/MADS/Demo/Characters/Mannequins/Meshes/SKM_Manny.SKM_Manny" :`1` "/Game/MADS/Demo/Characters/Mannequins/Meshes/SKM_Quinn.SKM_Quinn" :!type "SkeletalMesh Object Reference") true)
  (`SkeletalMeshComponent.SetAnimInstanceClass` _mesh (select `int` _chardata_gender :`0` "/Game/MADS/Demo/Characters/Mannequins/Animations/ABP_Manny.ABP_Manny_C" :`1` "/Game/MADS/Demo/Characters/Mannequins/Animations/ABP_Quinn.ABP_Quinn_C" :!type "Object Class Reference"))
  (for (_array_element _array_index) (`SkeletalMesh.Materials` (`SkeletalMeshComponent.GetSkeletalMeshAsset` (`self.Mesh`)))
    (`PrimitiveComponent.SetMaterial` _mesh _array_index (break `SkeletalMaterial` _array_element))))

(fn `StartRotation`
  (params (StartMouseRotation :type "Vector2D Structure"))
  (set `self.StartMouseRotation` StartMouseRotation)
  (set `self.EnableRotation` true))

(fn `UserConstructionScript`)