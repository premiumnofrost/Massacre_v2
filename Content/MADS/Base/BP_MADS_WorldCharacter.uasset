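; BP_MADS_WorldCharacter is a character Blueprint whose appearance and kill/death score come from its CharData struct.
; OnRep_CharData calls CustomChar, which applies the PersonToPlay skeletal mesh and the ABP_MACS anim class.
; ScoreAddKill and ScoreAddDeath increment the struct's score and pass it to UpdateCharacterScoreOnServer on the BP_MACS_PC controller's BPMADSComp.
; Gender-based mesh selection and dynamic-material tinting exist but are disconnected.
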(fn `CustomChar`
  (`self.SetMeshCharacter`))

(fn `OnRep_CharData`
  (`self.CustomChar`))

(fn `ScoreAddDeath`
  (bind (_chardata_id _chardata_owneraccountid _chardata_name _chardata_gender _chardata_color _chardata_level _chardata_transform _chardata_persontoplay _chardata_score) (break `/Game/MADS/DataModels/S_MADS_Character` (`self.CharData`)))
  (bind _chardata (`self.CharData`))
  (set `self.CharData` (make `/Game/MADS/DataModels/S_MADS_Character` (break `/Game/MADS/DataModels/S_MADS_Character` _chardata) (`.OwnerAccountID_30_CA7618D8473B1B09FED3DC88D9AD0E3A` (break `/Game/MADS/DataModels/S_MADS_Character` _chardata)) (`.Name_29_5B3F4456445AD44A05C72BAB17F026F6` (break `/Game/MADS/DataModels/S_MADS_Character` _chardata)) (`.Gender_19_2CAC573F43574E9664747D9D3D43291C` (break `/Game/MADS/DataModels/S_MADS_Character` _chardata)) (`.Color_22_A1A99F8B461E6D963DAFDB85705FD6F2` (break `/Game/MADS/DataModels/S_MADS_Character` _chardata)) (`.Level_25_C1BAB73741F2C20499B05D92B8D3DAC2` (break `/Game/MADS/DataModels/S_MADS_Character` _chardata)) (`.Transform_33_31C68FF740AAB84E379D5E9858E45685` (break `/Game/MADS/DataModels/S_MADS_Character` _chardata)) (`.PersonToPlay_36_F011B65C4270F1215C254CBD9591C421` (break `/Game/MADS/DataModels/S_MADS_Character` _chardata)) (make `/Game/MADS/DataModels/S_MADS_CharacterScore` (break `/Game/MADS/DataModels/S_MADS_CharacterScore` (`.Score_39_528F5DDF42328B0FB63EB9BA7E822FEB` (break `/Game/MADS/DataModels/S_MADS_Character` _chardata))) (+ (`.Deaths_42_B6E7C60B468A0303E82F7A9A572E878F` (break `/Game/MADS/DataModels/S_MADS_CharacterScore` (`.Score_39_528F5DDF42328B0FB63EB9BA7E822FEB` (break `/Game/MADS/DataModels/S_MADS_Character` _chardata)))) 1))))
  (bind _asbp_macs_pc (cast `/Game/MACS/Classes/BP_MACS_PC` (`self.GetController`)))
  (`/Game/MADS/Base/BP_MADS_Comp.UpdateCharacterScoreOnServer` (`/Game/MACS/Classes/BP_MACS_PC.BP_MADS_Comp` _asbp_macs_pc) _chardata_score)
  (return))

(fn `ScoreAddKill`
  (bind _chardata (`self.CharData`))
  (bind (_chardata_id _chardata_owneraccountid _chardata_name _chardata_gender _chardata_color _chardata_level _chardata_transform _chardata_persontoplay _chardata_score) (break `/Game/MADS/DataModels/S_MADS_Character` (`self.CharData`)))
  (set `self.CharData` (make `/Game/MADS/DataModels/S_MADS_Character` (break `/Game/MADS/DataModels/S_MADS_Character` _chardata) (`.OwnerAccountID_30_CA7618D8473B1B09FED3DC88D9AD0E3A` (break `/Game/MADS/DataModels/S_MADS_Character` _chardata)) (`.Name_29_5B3F4456445AD44A05C72BAB17F026F6` (break `/Game/MADS/DataModels/S_MADS_Character` _chardata)) (`.Gender_19_2CAC573F43574E9664747D9D3D43291C` (break `/Game/MADS/DataModels/S_MADS_Character` _chardata)) (`.Color_22_A1A99F8B461E6D963DAFDB85705FD6F2` (break `/Game/MADS/DataModels/S_MADS_Character` _chardata)) (`.Level_25_C1BAB73741F2C20499B05D92B8D3DAC2` (break `/Game/MADS/DataModels/S_MADS_Character` _chardata)) (`.Transform_33_31C68FF740AAB84E379D5E9858E45685` (break `/Game/MADS/DataModels/S_MADS_Character` _chardata)) (`.PersonToPlay_36_F011B65C4270F1215C254CBD9591C421` (break `/Game/MADS/DataModels/S_MADS_Character` _chardata)) (make `/Game/MADS/DataModels/S_MADS_CharacterScore` (+ (break `/Game/MADS/DataModels/S_MADS_CharacterScore` (`.Score_39_528F5DDF42328B0FB63EB9BA7E822FEB` (break `/Game/MADS/DataModels/S_MADS_Character` _chardata))) 1) (`.Deaths_42_B6E7C60B468A0303E82F7A9A572E878F` (break `/Game/MADS/DataModels/S_MADS_CharacterScore` (`.Score_39_528F5DDF42328B0FB63EB9BA7E822FEB` (break `/Game/MADS/DataModels/S_MADS_Character` _chardata)))))))
  (bind _asbp_macs_pc (cast `/Game/MACS/Classes/BP_MACS_PC` (`self.GetController`)))
  (`/Game/MADS/Base/BP_MADS_Comp.UpdateCharacterScoreOnServer` (`/Game/MACS/Classes/BP_MACS_PC.BP_MADS_Comp` _asbp_macs_pc) _chardata_score)
  (return))

(fn `SetMeshCharacter`
  (bind _mesh (`self.Mesh`))
  (bind (_chardata_id _chardata_owneraccountid _chardata_name _chardata_gender _chardata_color _chardata_level _chardata_transform _chardata_persontoplay) (break `/Game/MADS/DataModels/S_MADS_Character` (`self.CharData`)))
  ;[1 1 1] Set skeletal mesh
  (`SkinnedMeshComponent.SetSkinnedAssetAndUpdate` _mesh _chardata_persontoplay true)
  (`SkeletalMeshComponent.SetAnimInstanceClass` _mesh (select `int` _chardata_gender :`0` "/Game/MACS/Animations/ABP_MACS.ABP_MACS_C" :`1` "/Game/MACS/Animations/ABP_MACS.ABP_MACS_C" :!type "Object Class Reference")))

(fn `SetMeshColor`
  (bind (_chardata_id _chardata_owneraccountid _chardata_name _chardata_gender _chardata_color) (break `/Game/MADS/DataModels/S_MADS_Character` (`self.CharData`)))
  (bind _mesh (`self.Mesh`))
  (for (_array_element _array_index) (`MeshComponent.GetMaterials` _mesh)
    (bind _returnvalue (`PrimitiveComponent.CreateDynamicMaterialInstance` _mesh _array_index _array_element "None"))
    (`MaterialInstanceDynamic.SetVectorParameterValue` _returnvalue "Tint" _chardata_color)))

(fn `SetMeshGender`
  (bind _mesh (`self.Mesh`))
  (bind (_chardata_id _chardata_owneraccountid _chardata_name _chardata_gender) (break `/Game/MADS/DataModels/S_MADS_Character` (`self.CharData`)))
  ;[1 1 1] Set skeletal mesh and textures by gender
  (`SkinnedMeshComponent.SetSkinnedAssetAndUpdate` _mesh (select `int` _chardata_gender :`0` "/Game/MACS/Demo/ThirdPersonTemplateUE5/Characters/Mannequins/Meshes/SKM_Manny.SKM_Manny" :`1` "/Game/MACS/Demo/ThirdPersonTemplateUE5/Characters/Mannequins/Meshes/SKM_Manny.SKM_Manny" :!type "SkeletalMesh Object Reference") true)
  (`SkeletalMeshComponent.SetAnimInstanceClass` _mesh (select `int` _chardata_gender :`0` "/Game/MACS/Animations/ABP_MACS.ABP_MACS_C" :`1` "/Game/MACS/Animations/ABP_MACS.ABP_MACS_C" :!type "Object Class Reference"))
  (for (_array_element _array_index) (`SkeletalMesh.Materials` (`SkeletalMeshComponent.GetSkeletalMeshAsset` (`self.Mesh`)))
    (`PrimitiveComponent.SetMaterial` _mesh _array_index (break `SkeletalMaterial` _array_element))))

(fn `UserConstructionScript`)